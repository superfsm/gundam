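; BP_Matchmaker is an actor that automatically puts the player into a LAN multiplayer session when play begins.
; BeginPlay searches for LAN sessions and joins the first result if any are found.
; If the search returns none, it creates a four-connection LAN session and opens the LevelString level as a listen server.
; Only success outcomes are handled, so failed searches, creates or joins have no fallback.
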(event `self.ReceiveBeginPlay`
  (bind _results (`FindSessionsCallbackProxy.FindSessions` (`GameplayStatics.GetPlayerController` 0) 4 true)
    (:`OnSuccess`
      (if (== (`KismetArrayLibrary.Array_Length` _results) 0)
        (`CreateSessionCallbackProxy.CreateSession` (`GameplayStatics.GetPlayerController` 0) 4 true
          (:`OnSuccess`
            (`GameplayStatics.OpenLevel` (`self.LevelString`) true "listen")))
        (else
          (`JoinSessionCallbackProxy.JoinSession` (`GameplayStatics.GetPlayerController` 0) (`KismetArrayLibrary.Array_Get` _results)))))))

(event `self.ReceiveActorBeginOverlap`
  (params (OtherActor :type "Actor Object Reference")))

(event `self.ReceiveTick`
  (params (DeltaSeconds :type "Float (single-precision)")))

(fn `UserConstructionScript`)