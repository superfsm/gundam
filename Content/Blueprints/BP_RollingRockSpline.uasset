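; BP_RollingRockSpline builds a stone surface along an editable spline, apparently a track for rolling rocks.
; The construction script divides the spline length by Spacing and adds a collidable spline mesh per interval, plus one for the end.
; Each segment uses the RollingRockPlane1500 mesh with LightStone material, bent between world-space spline points using directions scaled by TangentScale.
; Segments use manual attachment, leaving them unattached so world-space coordinates apply directly.
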(fn `UserConstructionScript`
  (bind _tangent_scale (`self.Tangent Scale`))
  (bind _spline (`self.Spline`))
  (bind _spacing (`self.Spacing`))
  (for _index (range (+ (`.ReturnValue` (`KismetMathLibrary.FMod` (`SplineComponent.GetSplineLength` _spline) _spacing)) 1))
    (bind _returnvalue (`AddComponent|SplineMeshComponent_1074` :`bManualAttachment` true))
    (`PrimitiveComponent.SetCollisionEnabled` _returnvalue "QueryAndPhysics")
    (`StaticMeshComponent.SetStaticMesh` _returnvalue "/Game/Blueprints/RollingRockPlane1500.RollingRockPlane1500")
    (`PrimitiveComponent.SetMaterial` _returnvalue 0 "/Game/LayoutContent/BuildingBlock/LightStone.LightStone")
    (bind _returnvalue_2 (* _index _spacing))
    (bind _returnvalue_3 (+ _returnvalue_2 _spacing))
    (`SplineMeshComponent.SetStartAndEnd` _returnvalue (`SplineComponent.GetWorldLocationAtDistanceAlongSpline` _spline _returnvalue_2) (* (`SplineComponent.GetWorldDirectionAtDistanceAlongSpline` _spline _returnvalue_2) _tangent_scale) (`SplineComponent.GetWorldLocationAtDistanceAlongSpline` _spline _returnvalue_3) (* (`SplineComponent.GetWorldDirectionAtDistanceAlongSpline` _spline _returnvalue_3) _tangent_scale))))