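; Portal actor that teleports Gundam characters entering its sphere and removes itself after three uses.
; On sphere overlap, it checks for the exact GundamChar class and, on authority only, passes the character to the NetworkedGameInstance's Teleport function.
; A counter increments after each teleport call, and the portal destroys itself when it reaches the limit.
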(event `self.SphereCollision.OnComponentBeginOverlap`
  (params (OtherActor :type "Actor Object Reference") (OtherComp :type "PrimitiveComponent Object Reference") (OtherBodyIndex :type Integer) (bFromSweep :type Boolean) (SweepResult :type "EngineTypes.HitResult Structure (by ref)"))
  (if (== (`GameplayStatics.GetObjectClass` OtherActor) "/Game/Blueprints/GundamChar.GundamChar_C")
    (`/Engine/EditorBlueprintResources/ActorMacros.Switch Has Authority`
      (:`Authority`
        (bind _asnetworked_game_instance (cast `/Game/Blueprints/NetworkedGameInstance` (`GameplayStatics.GetGameInstance`)))
        (bind _asgundam_char (cast `/Game/Blueprints/GundamChar` OtherActor))
        (`/Game/Blueprints/NetworkedGameInstance.Teleport` _asnetworked_game_instance _asgundam_char)
        (bind _output_get (set `self.Count` (+ (`self.Count`) 1)))
        (if (== _output_get 3)
          (`self.K2_DestroyActor`))))))

(event `self.ReceiveBeginPlay`)

(event `self.ReceiveActorBeginOverlap`
  (params (OtherActor :type "Actor Object Reference")))

(event `self.ReceiveTick`
  (params (DeltaSeconds :type "Float (single-precision)")))

(fn `UserConstructionScript`)