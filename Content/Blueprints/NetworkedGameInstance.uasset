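; Game instance for a multiplayer Gundam game that manages online/LAN sessions and hosts shared gameplay events.
; Host creates a session and opens a listen level, Join takes the first result found and posts search status to BP_SessionJoiner, and Leave returns to the lobby.
; Helper events relay radar locations to other GundamChars, apply fixed hit damage, increment ScorePlayer counts, teleport to random Portals, and spawn brief explosions (named UpdateMaterial).
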(event `HostGameEvent`
  ;[1 1 1] Session
  (`CreateSessionCallbackProxy.CreateSession` (`GameplayStatics.GetPlayerController` 0) 4 (`self.UseLan?`)
    (:`OnSuccess`
      (`GameplayStatics.OpenLevel` (`self.LevelString`) true "listen"))))

(event `JoinGame`
  ;[1 1 1] Session
  (bind _results (`FindSessionsCallbackProxy.FindSessions` (`GameplayStatics.GetPlayerController` 0) 4 (`self.UseLan?`))
    (:`then`
      (bind _outactors (`GameplayStatics.GetAllActorsOfClass` "/Game/Blueprints/Old/BP_SessionJoiner.BP_SessionJoiner_C"))
      (for _array_element _outactors
        (`TextRenderComponent.SetText` (`/Game/Blueprints/Old/BP_SessionJoiner.Status Text` _array_element) "Searching for Sessions...")))
    (:`OnSuccess`
      (if (== (`KismetArrayLibrary.Array_Length` _results) 0)
        (bind _outactors_2 (`GameplayStatics.GetAllActorsOfClass` "/Game/Blueprints/Old/BP_SessionJoiner.BP_SessionJoiner_C"))
        (for _array_element_2 _outactors_2
          (`TextRenderComponent.SetText` (`/Game/Blueprints/Old/BP_SessionJoiner.Status Text` _array_element_2) "No Sessions Found"))
        (else
          (`JoinSessionCallbackProxy.JoinSession` (`GameplayStatics.GetPlayerController` 0) (`KismetArrayLibrary.Array_Get` _results)))))))

(event `LeaveGame`
  ;[1 1 1] Session
  (`DestroySessionCallbackProxy.DestroySession` (`GameplayStatics.GetPlayerController` 0)
    (:`OnSuccess`
      (`GameplayStatics.OpenLevel` (`self.LobbyLevelString`) true "listen"))))

(event `RadarUpdate`
  (params (RadarLocation :type "Object.Vector Structure" :default (0.0 0.0 0.0)) (Sender :type "/Game/Blueprints/GundamChar Object Reference"))
  ;[1 1 1] Radar Update
  (bind _outactors (`GameplayStatics.GetAllActorsOfClass` "/Game/Blueprints/GundamChar.GundamChar_C"))
  (for _array_element _outactors
    (if (!= _array_element Sender)
      (set `/Game/Blueprints/GundamChar.EnemyRadarLocation` RadarLocation _array_element))))

(event `CalculateHitDamage`
  (params (Actor :type "Actor Object Reference"))
  (bind _asgundam_char (cast `/Game/Blueprints/GundamChar` Actor))
  (set `/Game/Blueprints/GundamChar.Health` (- (`/Game/Blueprints/GundamChar.Health` _asgundam_char) 25.0) _asgundam_char))

(event `IncrementScore`
  (bind _outactors (`GameplayStatics.GetAllActorsOfClass` "/Game/Blueprints/ScorePlayer.ScorePlayer_C"))
  (for _array_element _outactors
    (bind _asscore_player (cast `/Game/Blueprints/ScorePlayer` _array_element))
    (set `/Game/Blueprints/ScorePlayer.Count` (+ (`/Game/Blueprints/ScorePlayer.Count` _asscore_player) 1) _asscore_player)))

(event `Teleport`
  (params (GundamChar :type "/Game/Blueprints/GundamChar Object Reference"))
  (bind _outactors (`GameplayStatics.GetAllActorsOfClass` "/Game/Blueprints/Portal.Portal_C"))
  (`Actor.K2_SetActorLocation` GundamChar (+ (`Actor.K2_GetActorLocation` (`KismetArrayLibrary.Array_Get` _outactors (`KismetMathLibrary.RandomIntegerInRange` 0 (- (`KismetArrayLibrary.Array_Length` _outactors) 1)))) (200.0 0.0 0.0)) false))

(event `UpdateMaterial`
  (params (Component :type "PrimitiveComponent Object Reference") (Location :type "Object.Vector Structure"))
  (bind _returnvalue (`GameplayStatics.SpawnEmitterAtLocation` "/Game/StarterContent/Particles/P_Explosion.P_Explosion" Location))
  (`KismetSystemLibrary.Delay` 0.2)
  (`ActorComponent.K2_DestroyComponent` _returnvalue))