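; BP_Swarm is a swarm projectile that can home in on a target's capsule and damages any GundamChar it hits.
; Capsule overlaps ignore the instigator and other swarm projectiles; any other actor triggers detonation.
; Tick also detonates it just before its lifespan expires.
; Detonation activates the explosion effect, zeroes velocity, swaps the launch audio for an explosion sound and destroys the actor after a short delay.
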(event `self.ReceiveBeginPlay`)

(event `self.ReceiveActorBeginOverlap`
  (params (OtherActor :type "Actor Object Reference")))

(event `self.ReceiveTick`
  (params (DeltaSeconds :type "Float (single-precision)"))
  (if (< (`self.GetLifeSpan`) 0.2)
    (`self.explode` :!label _label)
    (`KismetSystemLibrary.Delay` 0.2)
    (`self.K2_DestroyActor`)))

(event `self.Capsule.OnComponentBeginOverlap`
  (params (OtherActor :type "Actor Object Reference") (OtherComp :type "PrimitiveComponent Object Reference") (OtherBodyIndex :type Integer) (bFromSweep :type Boolean) (SweepResult :type "EngineTypes.HitResult Structure (by ref)"))
  (if (!= OtherActor (`self.GetInstigator`))
    (cast `/Game/Blueprints/BP_Swarm` OtherActor
      (:`CastFailed`
        (bind _asgundam_char (cast `/Game/Blueprints/GundamChar` OtherActor)
          (:`then`
            (`/Game/Blueprints/GundamChar.ModifyHealth` _asgundam_char -10.0)
            (goto _label))
          (:`CastFailed`
            (goto _label)))))))

(fn `explode`
  (bind _launch (`self.launch`))
  (`ActorComponent.SetActive` (`self.explosion`) true false)
  (`ProjectileMovementComponent.SetVelocityInLocalSpace` (`self.ProjectileMovement`) (0.0 0.0 0.0))
  (`AudioComponent.Stop` _launch)
  (`GameplayStatics.PlaySoundAttached` "/Game/StarterContent/Audio/Explosion01.Explosion01" _launch))

(fn `SetHoming`
  (params (Target :type "/Game/Blueprints/GundamChar Object Reference"))
  (bind _projectilemovement (`self.ProjectileMovement`))
  (set `ProjectileMovementComponent.HomingTargetComponent` (`Character.CapsuleComponent` Target) _projectilemovement)
  (set `ProjectileMovementComponent.bIsHomingProjectile` true _projectilemovement))

(fn `UserConstructionScript`)